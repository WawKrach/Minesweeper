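; Game mode Blueprint that shows a start menu on play and positions the player over the grid when the game starts.
; ToggleMenu creates the menu widget and binds to its GameStarted event, or removes and unbinds it if it exists.
; StartClicked closes the menu, then moves the player pawn to half the first BP_Grid's extent in X and Y, from GridSize and FieldSpace, at twice that height.
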(event Custom|ToggleMenu
  (Utilities|IsValid (Variables|Default|GetMenu)
    (:Is%20Valid
      (Widget|RemovefromParent (Variables|Default|GetMenu))
      (EventDispatchers|UnbindallEventsfromGameStarted (Variables|Default|GetMenu))
      (Variables|Default|SetMenu 0))
    (:Is%20Not%20Valid
      (bind _returnvalue (UserInterface|CreateWidget "/Game/Widgets/Menu.Menu_C"))
      (bind _output_get (Variables|Default|SetMenu _returnvalue))
      (UserInterface|Viewport|AddtoViewport _output_get 0)
      (EventDispatchers|BindEventtoGameStarted _output_get (EventDispatchers|CreateEvent :!event Custom|StartClicked)))))

(event Custom|StartClicked
  (Utilities|FlowControl|Sequence
    (:then_0
      (CallFunction|ToggleMenu))
    (:then_1
      (CallFunction|SetPlayerLocationwithGrid))))

(event EventBeginPlay
  (CallFunction|ToggleMenu))

(fn ConstructionScript)

(fn SetPlayerLocationwithGrid
  (bind _outactors (Actor|GetAllActorsOfClass "/Game/Blueprints/BP_Grid.BP_Grid_C"))
  (Transformation|SetActorLocation (Game|Player|GetPlayerPawn 0) (Math|Vector|MakeVector (* (/ (Variables|/Script/Minesweeper.Grid|GetGridSize (Utilities|Array|Get(acopy) _outactors)) 2) (Variables|/Script/Minesweeper.FieldStaticMeshComponent|GetFieldSpace (Actor|GetComponentbyClass (Utilities|Array|Get(acopy) _outactors) "/Script/Minesweeper.FieldStaticMeshComponent"))) (* (/ (Variables|/Script/Minesweeper.Grid|GetGridSize (Utilities|Array|Get(acopy) _outactors)) 2) (Variables|/Script/Minesweeper.FieldStaticMeshComponent|GetFieldSpace (Actor|GetComponentbyClass (Utilities|Array|Get(acopy) _outactors) "/Script/Minesweeper.FieldStaticMeshComponent"))) (* (* (/ (Variables|/Script/Minesweeper.Grid|GetGridSize (Utilities|Array|Get(acopy) _outactors)) 2) (Variables|/Script/Minesweeper.FieldStaticMeshComponent|GetFieldSpace (Actor|GetComponentbyClass (Utilities|Array|Get(acopy) _outactors) "/Script/Minesweeper.FieldStaticMeshComponent"))) 2.0)) false false))