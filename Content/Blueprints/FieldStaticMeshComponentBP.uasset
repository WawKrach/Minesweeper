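; Static mesh component for a single Minesweeper field that shows its current state through its material.
; Flag, unflag, reveal and reset events call the parent logic, then set the visual, with reveal deriving it from flag, mine and neighbor count.
; Each visual drives the UTail material scalar as an offset into a twelve-tile texture strip.
; Flagged and unrevealed currently map to the same tile.
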(event EventBeginPlay)

(event EventResetField
  (|CallParentFunction)
  (CallFunction|SetVisual "NewEnumerator5"))

(event EventShowFlag
  (|CallParentFunction)
  (CallFunction|SetVisual "NewEnumerator1"))

(event EventReveal
  (|CallParentFunction)
  (CallFunction|SetVisual (CallFunction|GetRevealedState)))

(event EventTakeFlag
  (|CallParentFunction)
  (CallFunction|SetVisual "NewEnumerator5"))

(fn SetVisual
  (params (VissualState :type Enum_VisualState%20Enum :default "NewEnumerator3"))
  (switch Utilities|FlowControl|Switch|SwitchonEnum_VisualState VissualState
    (:NewEnumerator5
      (Rendering|Material|SetScalarParameterValue (Variables|Default|GetFieldMaterial) "UTail" (CallFunction|FindSpaceonTexture 10) :!class /Script/Engine.MaterialInstanceDynamic))
    (:NewEnumerator3
      (Rendering|Material|SetScalarParameterValue (Variables|Default|GetFieldMaterial) "UTail" (CallFunction|FindSpaceonTexture) :!class /Script/Engine.MaterialInstanceDynamic))
    (:NewEnumerator1
      (Rendering|Material|SetScalarParameterValue (Variables|Default|GetFieldMaterial) "UTail" (CallFunction|FindSpaceonTexture 10) :!class /Script/Engine.MaterialInstanceDynamic))
    (:NewEnumerator2
      (Rendering|Material|SetScalarParameterValue (Variables|Default|GetFieldMaterial) "UTail" (CallFunction|FindSpaceonTexture 9) :!class /Script/Engine.MaterialInstanceDynamic))
    (:NewEnumerator4
      (Rendering|Material|SetScalarParameterValue (Variables|Default|GetFieldMaterial) "UTail" (CallFunction|FindSpaceonTexture (Variables|Default|GetNeightbourMinesCounter)) :!class /Script/Engine.MaterialInstanceDynamic))))

(fn GetRevealedState
  (Utilities|FlowControl|Sequence
    (:then_0
      (if (Math|Boolean|ANDBoolean (not (Variables|Default|GetbMined)) (not (Variables|Default|GetbFlaged)) (== (Variables|Default|GetNeightbourMinesCounter) 0))
        (return "NewEnumerator3")))
    (:then_1
      (if (Variables|Default|GetbFlaged)
        (return "NewEnumerator1")))
    (:then_2
      (if (Variables|Default|GetbMined)
        (return "NewEnumerator2")))
    (:then_3
      (if (!= (Variables|Default|GetNeightbourMinesCounter) 0)
        (return "NewEnumerator4")))))

(fn FindSpaceonTexture
  (params (USpaceOnTexture :type Integer))
  (return (+ (* USpaceOnTexture 0.083333) 0.0026)))